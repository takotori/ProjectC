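; Gameplay ability that reloads the owner's weapon through a reload montage.
; While active it holds a non-replicated NoFire loose tag on the owning actor, removed when the ability ends.
; A ReloadDone gameplay event, awaited alongside the montage, triggers the reload and ability end on authority only.
; Montage completion ends the ability locally, while interruption or cancellation ends it without reloading.
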(event Ability|EventActivateAbility
  (Utilities|FlowControl|Sequence
    (:then_0
      (Ability|GameplayEffect|AddLooseGameplayTags (Ability|GetOwningActorfromActorInfo) (GameplayTags|MakeLiteralGameplayTagContainer "(GameplayTags=((TagName=\"Ability.Weapon.NoFire\")))")))
    (:then_1
      (|PlayMontageandWaitProxy "None" (Variables|Default|GetReloadMontage) 1.0 "None" true 1.0 0.0
        (:then
          (Ability|Tasks|WaitGameplayEvent "(TagName=\"GameplayEvent.ReloadDone\")" 0 true
            (:EventReceived
              (Ability|HasAuthority
                (:True
                  (Class|ReloadAbility|ReloadWeapon)
                  (Ability|EndAbility))))))
        (:OnCompleted
          (Ability|EndAbilityLocally))
        (:OnInterrupted
          (Ability|EndAbility :!label _label))
        (:OnCancelled
          (goto _label))))))

(event Ability|EventOnEndAbility
  (params (bWasCancelled :type Boolean))
  (|CallParentFunction bWasCancelled)
  (Ability|GameplayEffect|RemoveLooseGameplayTags (Ability|GetOwningActorfromActorInfo) (GameplayTags|MakeLiteralGameplayTagContainer "(GameplayTags=((TagName=\"Ability.Weapon.NoFire\")))")))