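; GA_Fire is the default ranged weapon fire ability, which triggers a reload instead when ammo is out.
; On activation the locally controlled player starts targeting while the fire montage plays, with a short timer or montage interruption ending the ability.
; The montage keeps playing after the ability ends.
; Incoming target data applies the ammo consumption effect to the owner and passes the data to UseAbility.
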(event Custom|FireComplete
  (Ability|EndAbility))

(event EventActivateLocalPlayerAbility
  (bind _returnvalue (Class|FireAbility|HasEnoughAmmo))
  (if _returnvalue
    (Utilities|FlowControl|Sequence
      (:then_0
        (Pawn|IsLocallyControlled
          (:True
            (Class|FireAbility|StartRangedWeaponTargeting))))
      (:then_1
        (|PlayMontageandWaitProxy "None" (Variables|Default|GetFireMontage) 1.0 "None" false 1.0 0.0
          (:then
            (Utilities|Time|SetTimerbyEvent (EventDispatchers|CreateEvent :!event Custom|FireComplete) 0.15))
          (:OnInterrupted
            (Ability|EndAbility :!label _label))
          (:OnCancelled
            (goto _label)))))
    (else
      (Abilities|TryActivateAbilitybyClass (Ability|GetAbilitySystemComponentfromActorInfo) "/Game/Blueprints/Abilities/DefaultAbilities/GA_Reload.GA_Reload_C" true)
      (goto _label))))

(event EventActivateAbilitywithTargetData
  (params (InData :type Gameplay%20Ability%20Target%20Data%20Handle%20Structure%20%28by%20ref%29) (ApplicationTag :type Gameplay%20Tag%20Structure))
  (Ability|ApplyGameplayEffectToOwner "/Game/Blueprints/Abilities/DefaultEffects/GE_AmmoConsumption.GE_AmmoConsumption_C")
  (Class|FireAbility|UseAbility InData ApplicationTag))